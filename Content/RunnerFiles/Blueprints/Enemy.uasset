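; Enemy actor for the runner game that moves along a set path and kills the player on contact.
; On BeginPlay it records its start location and plays a timeline that lerps its static mesh between that point and an EndPoint offset.
; On overlap with the PlayerCharacter, it calls the player's DeathFunction unless the ThirdPersonGameMode's IsWalkThroughWalls flag is set.
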(event `self.ReceiveBeginPlay`
  (set `self.StartingPoint` (`self.K2_GetActorLocation`))
  (bind (_direction _newtrack_1) (`Timeline|TimelineMovement`)
    (:`Update`
      (`SceneComponent.K2_SetWorldLocation` (`self.StaticMesh`) (`KismetMathLibrary.VLerp` (`self.StartingPoint`) (+ (`self.StartingPoint`) (`self.EndPoint`)) _newtrack_1) false false))))

(event `self.ReceiveActorBeginOverlap`
  (params (OtherActor :type "Actor Object Reference"))
  (bind _asplayer_character (cast `/Game/ThirdPersonBP/Blueprints/PlayerCharacter` OtherActor))
  (bind _asthird_person_game_mode (cast `/Game/ThirdPersonBP/Blueprints/ThirdPersonGameMode` (`GameplayStatics.GetGameMode`)))
  (if (not (`/Game/ThirdPersonBP/Blueprints/ThirdPersonGameMode.isWalkThroughWalls` _asthird_person_game_mode))
    (`/Game/ThirdPersonBP/Blueprints/PlayerCharacter.DeathFunction` _asplayer_character)))

(event `self.ReceiveTick`
  (params (DeltaSeconds :type "Float (single-precision)")))

(fn `UserConstructionScript`)