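; BoostCube is a runner pickup that grants the player a temporary walk-through-walls boost on overlap.
; It sets the flag and duration on ThirdPersonGameMode, plays a coin sound, hides itself, then clears both and destroys itself after ten seconds.
; Each cube's Tick uses a Delay to decrement the shared duration roughly every second.
; Cubes also self-destroy a minute after spawning.
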(event `self.ReceiveBeginPlay`
  ;[1 1 1] Удаляем с карты после прохождения
  (`KismetSystemLibrary.Delay` 60.0)
  (`self.K2_DestroyActor`))

(event `self.ReceiveActorBeginOverlap`
  (params (OtherActor :type "Actor Object Reference"))
  (cast `/Game/ThirdPersonBP/Blueprints/PlayerCharacter` OtherActor)
  (bind _asthird_person_game_mode (cast `/Game/ThirdPersonBP/Blueprints/ThirdPersonGameMode` (`GameplayStatics.GetGameMode`)))
  (set `/Game/ThirdPersonBP/Blueprints/ThirdPersonGameMode.isWalkThroughWalls` true _asthird_person_game_mode)
  (set `/Game/ThirdPersonBP/Blueprints/ThirdPersonGameMode.WalkDuration` 10 _asthird_person_game_mode)
  (`GameplayStatics.SpawnSound2D` "/Game/RunnerFiles/Sounds/Pickup_Coin_Sound.Pickup_Coin_Sound" 1.0 1.0 0.0 null)
  (`self.SetActorHiddenInGame` true)
  (`KismetSystemLibrary.RetriggerableDelay` 10.0)
  (set `/Game/ThirdPersonBP/Blueprints/ThirdPersonGameMode.isWalkThroughWalls` false _asthird_person_game_mode)
  (set `/Game/ThirdPersonBP/Blueprints/ThirdPersonGameMode.WalkDuration` 0 _asthird_person_game_mode)
  (`self.K2_DestroyActor`))

(event `self.ReceiveTick`
  (params (DeltaSeconds :type "Float (single-precision)"))
  (`KismetSystemLibrary.Delay` 1.0)
  (bind _asthird_person_game_mode (cast `/Game/ThirdPersonBP/Blueprints/ThirdPersonGameMode` (`GameplayStatics.GetGameMode`)))
  (bind _walkduration (`/Game/ThirdPersonBP/Blueprints/ThirdPersonGameMode.WalkDuration` _asthird_person_game_mode))
  (if (> _walkduration 0)
    (set `/Game/ThirdPersonBP/Blueprints/ThirdPersonGameMode.WalkDuration` (- _walkduration 1) _asthird_person_game_mode)))

(fn `UserConstructionScript`)