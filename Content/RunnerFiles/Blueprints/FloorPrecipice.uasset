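; Endless-runner precipice floor tile that spawns lane contents on BeginPlay and kills the player on hitting JumpEnd.
; SpawnObstacles chains three lanes through fresh random rolls for tree, rock, coin or boost cube; an empty lane skips those after it.
; When the player overlaps Box1, it asks the game mode for another tile, adds distance, raises clamped walk speed and destroys itself after a delay.
; BoostClock spawns are unconnected.
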(event `self.ReceiveBeginPlay`
  (`self.SpawnObstacles`))

(event `self.Box1.OnComponentBeginOverlap`
  (params (OverlappedComponent :type "PrimitiveComponent Object Reference") (OtherActor :type "Actor Object Reference") (OtherComp :type "PrimitiveComponent Object Reference") (OtherBodyIndex :type Integer) (bFromSweep :type Boolean) (SweepResult :type "HitResult Structure (by ref)"))
  (cast `/Game/ThirdPersonBP/Blueprints/ThirdPersonCharacter` OtherActor)
  (bind _asthird_person_game_mode (cast `/Game/ThirdPersonBP/Blueprints/ThirdPersonGameMode` (`GameplayStatics.GetGameMode`)))
  (`/Game/ThirdPersonBP/Blueprints/ThirdPersonGameMode.SpawnTile` _asthird_person_game_mode)
  (bind _asthird_person_game_mode_2 (cast `/Game/ThirdPersonBP/Blueprints/ThirdPersonGameMode` (`GameplayStatics.GetGameMode`)))
  (set `/Game/ThirdPersonBP/Blueprints/ThirdPersonGameMode.CurrentDistance` (+ (* 1 (`/Game/ThirdPersonBP/Blueprints/ThirdPersonGameMode.DistanceMultiplier` _asthird_person_game_mode_2)) (`/Game/ThirdPersonBP/Blueprints/ThirdPersonGameMode.CurrentDistance` _asthird_person_game_mode_2)) _asthird_person_game_mode_2)
  (bind _asthird_person_character (cast `/Game/ThirdPersonBP/Blueprints/ThirdPersonCharacter` (`GameplayStatics.GetPlayerCharacter` 0)))
  (bind _charactermovement (`Character.CharacterMovement` _asthird_person_character))
  (set `CharacterMovementComponent.MaxWalkSpeed` (`KismetMathLibrary.FClamp` (* (`CharacterMovementComponent.MaxWalkSpeed` _charactermovement) 1.03) 600.0 1800.0) _charactermovement)
  (`KismetSystemLibrary.Delay` 0.5)
  (`self.K2_DestroyActor`))

(event `self.JumpEnd.OnComponentHit`
  (params (HitComponent :type "PrimitiveComponent Object Reference") (OtherActor :type "Actor Object Reference") (OtherComp :type "PrimitiveComponent Object Reference") (NormalImpulse :type "Vector Structure") (Hit :type "HitResult Structure (by ref)"))
  (bind _asthird_person_character (cast `/Game/ThirdPersonBP/Blueprints/ThirdPersonCharacter` OtherActor))
  (`/Game/ThirdPersonBP/Blueprints/ThirdPersonCharacter.DeathFunction` _asthird_person_character))

(fn `SpawnObstacles`
  (bind _returnvalue (`KismetMathLibrary.RandomFloatInRange` 0.0 1.0))
  (bind _returnvalue_2 (`KismetMathLibrary.RandomFloatInRange` 0.0 1.0))
  (bind _returnvalue_3 (`KismetMathLibrary.RandomFloatInRange` 0.0 1.0))
  (bind _returnvalue_4 (`SceneComponent.K2_GetComponentToWorld` (`self.Lane0`)))
  (bind _returnvalue_5 (`SceneComponent.K2_GetComponentToWorld` (`self.Lane1`)))
  (bind _returnvalue_6 (`SceneComponent.K2_GetComponentToWorld` (`self.Lane2`)))
  ;[1 1 1] Left Lane
  (if (`KismetMathLibrary.InRange_FloatFloat` _returnvalue_2 0.0 0.4)
    (`|SpawnActorFromClass` "/Game/RunnerFiles/Blueprints/Tree.Tree_C" _returnvalue_4 "Undefined" "OverrideRootScale" null null)
    ;[1 1 1] Center Lane
    (if (`KismetMathLibrary.InRange_FloatFloat` _returnvalue_3 0.0 0.4) :!label _label
      (`|SpawnActorFromClass` "/Game/RunnerFiles/Blueprints/Tree.Tree_C" _returnvalue_5 "Undefined" "OverrideRootScale" null null)
      ;[1 1 1] Right Lane
      (if (`KismetMathLibrary.InRange_FloatFloat` _returnvalue 0.0 0.4) :!label _label_2
        (`|SpawnActorFromClass` "/Game/RunnerFiles/Blueprints/Tree.Tree_C" _returnvalue_6 "Undefined" "OverrideRootScale" null null)
        (elif (`KismetMathLibrary.InRange_FloatFloat` _returnvalue 0.4 0.5)
          (`|SpawnActorFromClass` "/Game/RunnerFiles/Blueprints/ObstacleRock.ObstacleRock_C" _returnvalue_6 "Undefined" "OverrideRootScale" null null)
          (elif (`KismetMathLibrary.InRange_FloatFloat` _returnvalue 0.5 0.9)
            (`|SpawnActorFromClass` "/Game/RunnerFiles/Blueprints/CoinPickup.CoinPickup_C" _returnvalue_6 "Undefined" "OverrideRootScale" null null)
            (elif (`KismetMathLibrary.InRange_FloatFloat` _returnvalue 0.9)
              (`|SpawnActorFromClass` "/Game/RunnerFiles/Blueprints/BoostCube.BoostCube_C" _returnvalue_6 "Undefined" "OverrideRootScale" null null)))))
      (elif (`KismetMathLibrary.InRange_FloatFloat` _returnvalue_3 0.4 0.5)
        (`|SpawnActorFromClass` "/Game/RunnerFiles/Blueprints/ObstacleRock.ObstacleRock_C" _returnvalue_5 "Undefined" "OverrideRootScale" null null)
        (goto _label_2)
        (elif (`KismetMathLibrary.InRange_FloatFloat` _returnvalue_3 0.5 0.9)
          (`|SpawnActorFromClass` "/Game/RunnerFiles/Blueprints/CoinPickup.CoinPickup_C" _returnvalue_5 "Undefined" "OverrideRootScale" null null)
          (goto _label_2)
          (elif (`KismetMathLibrary.InRange_FloatFloat` _returnvalue_3 0.9)
            (`|SpawnActorFromClass` "/Game/RunnerFiles/Blueprints/BoostCube.BoostCube_C" _returnvalue_5 "Undefined" "OverrideRootScale" null null)
            (goto _label_2)))))
    (elif (`KismetMathLibrary.InRange_FloatFloat` _returnvalue_2 0.4 0.5)
      (`|SpawnActorFromClass` "/Game/RunnerFiles/Blueprints/ObstacleRock.ObstacleRock_C" _returnvalue_4 "Undefined" "OverrideRootScale" null null)
      (goto _label)
      (elif (`KismetMathLibrary.InRange_FloatFloat` _returnvalue_2 0.5 0.9)
        (`|SpawnActorFromClass` "/Game/RunnerFiles/Blueprints/CoinPickup.CoinPickup_C" _returnvalue_4 "Undefined" "OverrideRootScale" null null)
        (goto _label)
        (elif (`KismetMathLibrary.InRange_FloatFloat` _returnvalue_2 0.9)
          (`|SpawnActorFromClass` "/Game/RunnerFiles/Blueprints/BoostCube.BoostCube_C" _returnvalue_4 "Undefined" "OverrideRootScale" null null)
          (goto _label))))))

(fn `UserConstructionScript`)