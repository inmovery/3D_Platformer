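; Endless runner floor tile, named FloorAbyss, with a box that kills the player on overlap.
; On BeginPlay it randomly fills left, middle and right lanes with enemies, rocks, coins or boosts, rolling each lane only if the previous one spawned something.
; Its end trigger advances the game mode's platform count and distance, starts a new level every tenth platform, spawns the next tile, then destroys itself after a short delay.
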(event `self.ReceiveBeginPlay`
  (`self.SpawnObstacles`))

(event `self.EndTrigger.OnComponentBeginOverlap`
  (params (OverlappedComponent :type "PrimitiveComponent Object Reference") (OtherActor :type "Actor Object Reference") (OtherComp :type "PrimitiveComponent Object Reference") (OtherBodyIndex :type Integer) (bFromSweep :type Boolean) (SweepResult :type "HitResult Structure (by ref)"))
  (cast `/Game/ThirdPersonBP/Blueprints/PlayerCharacter` OtherActor)
  (bind _asthird_person_game_mode (cast `/Game/ThirdPersonBP/Blueprints/ThirdPersonGameMode` (`GameplayStatics.GetGameMode`)))
  ;[1 1 1] Проверка нового уровня (каждых новых 10 платформ)
  (bind _output_get (set `/Game/ThirdPersonBP/Blueprints/ThirdPersonGameMode.PassedPlatforms` (+ (`/Game/ThirdPersonBP/Blueprints/ThirdPersonGameMode.PassedPlatforms` _asthird_person_game_mode) 1) _asthird_person_game_mode))
  (if (== (mod _output_get 10) 0)
    (`/Game/ThirdPersonBP/Blueprints/ThirdPersonGameMode.NewLevel` _asthird_person_game_mode))
  (`/Game/ThirdPersonBP/Blueprints/ThirdPersonGameMode.Spawn Tile` _asthird_person_game_mode)
  (bind _asthird_person_game_mode_2 (cast `/Game/ThirdPersonBP/Blueprints/ThirdPersonGameMode` (`GameplayStatics.GetGameMode`)))
  (set `/Game/ThirdPersonBP/Blueprints/ThirdPersonGameMode.CurrentDistance` (+ (* 1 (`/Game/ThirdPersonBP/Blueprints/ThirdPersonGameMode.DistanceMultiplier` _asthird_person_game_mode_2)) (`/Game/ThirdPersonBP/Blueprints/ThirdPersonGameMode.CurrentDistance` _asthird_person_game_mode_2)) _asthird_person_game_mode_2)
  (`KismetSystemLibrary.Delay` 0.5)
  (`self.K2_DestroyActor`))

(event `self.Box.OnComponentBeginOverlap`
  (params (OverlappedComponent :type "PrimitiveComponent Object Reference") (OtherActor :type "Actor Object Reference") (OtherComp :type "PrimitiveComponent Object Reference") (OtherBodyIndex :type Integer) (bFromSweep :type Boolean) (SweepResult :type "HitResult Structure (by ref)"))
  (bind _asplayer_character (cast `/Game/ThirdPersonBP/Blueprints/PlayerCharacter` OtherActor))
  (`/Game/ThirdPersonBP/Blueprints/PlayerCharacter.DeathFunction` _asplayer_character))

(fn `SpawnObstacles`
  (bind _returnvalue (`KismetMathLibrary.RandomFloatInRange` 0.0 1.0))
  (bind _returnvalue_2 (`KismetMathLibrary.RandomFloatInRange` 0.0 1.0))
  (bind _returnvalue_3 (`SceneComponent.K2_GetComponentToWorld` (`self.LeftLane`)))
  (bind _returnvalue_4 (`SceneComponent.K2_GetComponentToWorld` (`self.MiddleLane`)))
  (bind _returnvalue_5 (`SceneComponent.K2_GetComponentToWorld` (`self.RightLane`)))
  ;[1 1 1] Left Lane
  (switch `int` (`KismetMathLibrary.RandomIntegerInRange` 0 5)
    (:`1`
      (if (`KismetMathLibrary.InRange_FloatFloat` (`KismetMathLibrary.RandomFloatInRange` 0.0 1.0) 0.0 0.6)
        (`|SpawnActorFromClass` "/Game/RunnerFiles/Blueprints/Enemy.Enemy_C" _returnvalue_3 "Undefined" "OverrideRootScale" null null)
        ;[1 1 1] Center Lane
        (if (`KismetMathLibrary.InRange_FloatFloat` _returnvalue_2 0.0 0.4) :!label _label
          (`|SpawnActorFromClass` "/Game/RunnerFiles/Blueprints/Enemy.Enemy_C" _returnvalue_4 "Undefined" "OverrideRootScale" null null)
          ;[1 1 1] Right Lane
          (if (`KismetMathLibrary.InRange_FloatFloat` _returnvalue 0.0 0.4) :!label _label_2
            (`|SpawnActorFromClass` "/Game/RunnerFiles/Blueprints/Enemy.Enemy_C" _returnvalue_5 "Undefined" "OverrideRootScale" null null)
            (elif (`KismetMathLibrary.InRange_FloatFloat` _returnvalue 0.4 0.5)
              (`|SpawnActorFromClass` "/Game/RunnerFiles/Blueprints/Rock.Rock_C" _returnvalue_5 "Undefined" "OverrideRootScale" null null)
              (elif (`KismetMathLibrary.InRange_FloatFloat` _returnvalue 0.5 0.9)
                (`|SpawnActorFromClass` "/Game/RunnerFiles/Blueprints/Coin.Coin_C" _returnvalue_5 "Undefined" "OverrideRootScale" null null)
                (elif (`KismetMathLibrary.InRange_FloatFloat` _returnvalue 0.9)
                  (`|SpawnActorFromClass` "/Game/RunnerFiles/Blueprints/BoostCube.BoostCube_C" _returnvalue_5 "Undefined" "OverrideRootScale" null null)))))
          (elif (`KismetMathLibrary.InRange_FloatFloat` _returnvalue_2 0.4 0.5)
            (`|SpawnActorFromClass` "/Game/RunnerFiles/Blueprints/Rock.Rock_C" _returnvalue_4 "Undefined" "OverrideRootScale" null null)
            (goto _label_2)
            (elif (`KismetMathLibrary.InRange_FloatFloat` _returnvalue_2 0.5 0.9)
              (`|SpawnActorFromClass` "/Game/RunnerFiles/Blueprints/Coin.Coin_C" _returnvalue_4 "Undefined" "OverrideRootScale" null null)
              (goto _label_2)
              (elif (`KismetMathLibrary.InRange_FloatFloat` _returnvalue_2 0.9)
                (`|SpawnActorFromClass` "/Game/RunnerFiles/Blueprints/BoostCube.BoostCube_C" _returnvalue_4 "Undefined" "OverrideRootScale" null null)
                (goto _label_2)))))))
    (:`2`
      (if (`KismetMathLibrary.InRange_FloatFloat` (`KismetMathLibrary.RandomFloatInRange` 0.0 1.0) 0.0 0.6)
        (`|SpawnActorFromClass` "/Game/RunnerFiles/Blueprints/Rock.Rock_C" _returnvalue_3 "Undefined" "OverrideRootScale" null null)
        (goto _label)))
    (:`3`
      (if (`KismetMathLibrary.InRange_FloatFloat` (`KismetMathLibrary.RandomFloatInRange` 0.0 1.0) 0.0 0.6)
        (`|SpawnActorFromClass` "/Game/RunnerFiles/Blueprints/Coin.Coin_C" _returnvalue_3 "Undefined" "OverrideRootScale" null null)
        (goto _label)))
    (:`5`
      (switch `int` (`KismetMathLibrary.RandomIntegerInRange` 0 3)
        (:`1`
          (`|SpawnActorFromClass` "/Game/RunnerFiles/Blueprints/BoostCube.BoostCube_C" _returnvalue_3 "Undefined" "OverrideRootScale" null null)
          (goto _label))
        (:`2`
          (`|SpawnActorFromClass` "/Game/RunnerFiles/Blueprints/BoostClock.BoostClock_C" _returnvalue_3 "Undefined" "OverrideRootScale" null null)
          (goto _label))))))

(fn `UserConstructionScript`)